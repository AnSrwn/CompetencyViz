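; Player pawn for an Android ARCore app that places a world anchor and drags tag actors, with axis-driven movement and look for web.
; Touch traces tracked geometry to spawn a pinned BP_AnchorActor.
; Gates allow one successful placement and debug-draw detected geometry until then.
; MoveTagActor stores grab distance, so touch moves reposition the object along the deprojected screen ray until StopMovingTagActor.
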(event Custom|AnchorActorSpawned
  ;[1 0 0 0.5] Get Ar planes
  (Utilities|FlowControl|Gate false) ; enters at Close
)

(event EventBeginPlay
  ;[1 0 0 0.5] Start AR Session
  (switch string (Game|GetPlatformName)
    (:Android
      (Class|ARBlueprintLibrary|StartARSession "/Game/D_SessionConfig.D_SessionConfig"))))

(event EventTick
  (params (DeltaSeconds :type Float%20%28single-precision%29))
  ;[1 0 0 0.5] Get Ar planes
  (Utilities|FlowControl|Gate false
    (:Exit
      (switch string (Game|GetPlatformName)
        (:Android
          (bind _returnvalue (Class|ARBlueprintLibrary|GetAllGeometries))
          (for _array_element _returnvalue
            (Class|ARBlueprintLibrary|DebugDrawTrackedGeometry _array_element "(R=1.000000,G=0.103198,B=0.143001,A=0.750000)")))))))

(event Input|AxisEvents|InputAxisForward
  (params (AxisValue :type Float%20%28single-precision%29))
  (bind _returnvalue (Pawn|GetControlRotation :!class /Script/Engine.Pawn))
  ;[0 1 0 0.5] Pawn Movement for Web
  (Pawn|Input|AddMovementInput (Math|Vector|GetForwardVector (Math|Rotator|MakeRotator (.roll _returnvalue) (.pitch _returnvalue) (.yaw _returnvalue))) AxisValue false))

(event Input|AxisEvents|InputAxisRight
  (params (AxisValue :type Float%20%28single-precision%29))
  (bind _returnvalue (Pawn|GetControlRotation :!class /Script/Engine.Pawn))
  ;[0 1 0 0.5] Pawn Movement for Web
  (Pawn|Input|AddMovementInput (Math|Vector|GetRightVector (Math|Rotator|MakeRotator (.roll _returnvalue) (.pitch _returnvalue) (.yaw _returnvalue))) AxisValue false))

(event Input|AxisEvents|InputAxisTurn
  (params (AxisValue :type Float%20%28single-precision%29))
  ;[0 1 0 0.5] Pawn Movement for Web
  (Pawn|Input|AddControllerYawInput AxisValue))

(event Input|AxisEvents|InputAxisLookup
  (params (AxisValue :type Float%20%28single-precision%29))
  ;[0 1 0 0.5] Pawn Movement for Web
  (Pawn|Input|AddControllerPitchInput AxisValue))

(event Input|TouchEvents|InputTouch
  (params (Location :type Vector) (FingerIndex :type ETouchIndex%20Enum))
  (bind _returnvalue (Game|GetPlayerController 0))
  (bind _returnvalue_2 (Game|GetPlayerController 0))
  (bind (_locationx _locationy) (Class|PlayerController|GetInputTouchState _returnvalue_2 FingerIndex))
  (bind (_locationx_2 _locationy_2) (Class|PlayerController|GetInputTouchState _returnvalue FingerIndex))
  (bind _returnvalue_3 (Math|Vector2D|MakeVector2D _locationx_2 _locationy_2))
  ;[1 0 0 0.5] Place AnchorActorInWorld
  (:Pressed
    (switch string (Game|GetPlatformName)
      (:Android
        (Utilities|FlowControl|Gate false :!label _label
          (:Exit
            (bind (_outhitresults _returnvalue_4) (Class|GoogleARCoreFrameFunctionLibrary|ARCoreLineTrace _returnvalue_3 (Variables|Default|GetARCoreLineTraceChannels)))
            (if _returnvalue_4
              (if (Utilities|IsHittingFrontSurface (Utilities|Array|Get(acopy) _outhitresults) _returnvalue _returnvalue_3)
                (bind _result (CallFunction|SpawnAnchorActor (Utilities|Array|Get(acopy) _outhitresults)))
                (if _result
                  (CallFunction|AnchorActorSpawned)
                  (goto _label Close)
                  (else
                    (Development|PrintString "Failed to place Anchor")))
                (else
                  (Development|PrintString "is not hitting front surface")))
              (else
                (Development|PrintString "no hit result"))))))))
  (:Moved
    (if (Variables|Default|GetObjectIsGrabbed)
      (Transformation|SetActorLocation (Variables|Default|GetGrabbedObject) (+ (* (Math|Vector|Normalize (.WorldDirection (Class|PlayerController|DeprojectScreenPositiontoWorld _returnvalue_2 _locationx _locationy))) (Variables|Default|GetDistanceToGrabbedObject)) (Variables|/Script/Engine.SceneComponent|GetRelativeLocation (Variables|Default|GetCamera))) false false))))

(fn ConstructionScript)

(fn WorldHitTest
  (params (ScreenPosition :type Vector%202D%20Structure))
  (bind _returnvalue (Game|GetPlayerController 0))
  (bind (_worldposition _worlddirection) (Class|GameplayStatics|DeprojectScreentoWorld _returnvalue ScreenPosition))
  (bind (_outhit _returnvalue_2) (Collision|LineTraceForObjects _worldposition (+ _worldposition (* _worlddirection 1000)) (Utilities|Array|MakeArray "ObjectTypeQuery1" "ObjectTypeQuery2" "ObjectTypeQuery3" "ObjectTypeQuery4" "ObjectTypeQuery5" "ObjectTypeQuery6") false 0 "None"))
  (return _outhit _returnvalue_2))

(fn SpawnAnchorActor
  (params (HitTestResult :type AR%20Trace%20Result%20Structure%20%28by%20ref%29))
  (bind _returnvalue (Class|ARBlueprintLibrary|PinComponent 0 (Class|ARTraceResultLibrary|GetLocaltoWorldTransform HitTestResult) (Class|ARTraceResultLibrary|GetTrackedGeometry HitTestResult)))
  (if (Utilities|IsValid _returnvalue)
    (bind _returnvalue_2 (Game|SpawnActorfromClass "/Game/Blueprints/BP_AnchorActor.BP_AnchorActor_C" (Class|ARPin|GetLocaltoWorldTransform _returnvalue) "Undefined" 0 0))
    (Default|AssignARPin _returnvalue_2 _returnvalue)
    (return true)
    (else
      (return false))))

(fn MoveTagActor
  (params (TagActor :type BP%20Tag%20Actor%20Object%20Reference))
  (bind _camera (Variables|Default|GetCamera))
  (bind _relativelocation (Variables|/Script/Engine.SceneComponent|GetRelativeLocation _camera))
  (bind _output_get (Variables|Default|SetGrabbedObject TagActor))
  (Variables|Default|SetDistanceToGrabbedObject (Math|Vector|VectorLength (- (Transformation|GetWorldLocation (Variables|/Game/Blueprints/BP_TagActor.BP_TagActor_C|GetDefaultSceneRoot _output_get)) (Transformation|GetWorldLocation (Variables|Default|GetCamera)))))
  (Transformation|SetRelativeLocation (Variables|Default|GetGrabbedObjectLocation) (Math|Vector|MakeVector (+ (.x _relativelocation) (Math|Vector|VectorLength (- (Transformation|GetWorldLocation (Variables|/Game/Blueprints/BP_TagActor.BP_TagActor_C|GetDefaultSceneRoot _output_get)) (Transformation|GetWorldLocation (Variables|Default|GetCamera))))) (.y _relativelocation) (.z _relativelocation)) false false)
  (Variables|Default|SetObjectIsGrabbed true))

(fn StopMovingTagActor
  (Variables|Default|SetObjectIsGrabbed false))