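; Blueprint function library that converts DateTime values to and from ISO 8601-style strings ending in "Z".
; DateTimeToString appends the date and time components down to milliseconds, without zero padding or timezone conversion.
; StringToDateTime reverses this by splitting on "T", stripping "Z" and parsing the delimited parts as integers.
; Parsing has no validation and relies on a "." before the milliseconds to extract the time fields.
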(fn DateTimetoString
  (params (DateTime :type Date%20Time%20Structure))
  (return (Utilities|String|Append (Utilities|String|MakeLiteralString (Utilities|String|ToString(Integer) (.year DateTime))) "-" (Utilities|String|ToString(Integer) (.month DateTime)) "-" (Utilities|String|ToString(Integer) (.day DateTime)) "T" (Utilities|String|ToString(Integer) (.hour DateTime)) ":" (Utilities|String|ToString(Integer) (.minute DateTime)) ":" (Utilities|String|ToString(Integer) (.second DateTime)) "." (Utilities|String|ToString(Integer) (.millisecond DateTime)) "Z")))

(fn StringtoDateTime
  (params (DateTime :type String))
  (bind (_lefts _rights) (Utilities|String|Split DateTime "T"))
  (bind _returnvalue (Utilities|String|ParseIntoArray _lefts "-"))
  (bind _returnvalue_2 (Utilities|String|Replace _rights "Z"))
  (bind (_lefts_2 _rights_2) (Utilities|String|Split _returnvalue_2 "."))
  (bind _returnvalue_3 (Utilities|String|ParseIntoArray _lefts_2 ":"))
  (return (Math|DateTime|MakeDateTime (Math|Conversions|ToInteger(Byte) (Utilities|Array|Get(acopy) _returnvalue)) (Math|Conversions|ToInteger(Byte) (Utilities|Array|Get(acopy) _returnvalue 1)) (Math|Conversions|ToInteger(Byte) (Utilities|Array|Get(acopy) _returnvalue 2)) (Math|Conversions|ToInteger(Byte) (Utilities|Array|Get(acopy) _returnvalue_3)) (Math|Conversions|ToInteger(Byte) (Utilities|Array|Get(acopy) _returnvalue_3 1)) (Math|Conversions|ToInteger(Byte) (Utilities|Array|Get(acopy) _returnvalue_3 2)) (Math|Conversions|ToInteger(Byte) _rights_2))))