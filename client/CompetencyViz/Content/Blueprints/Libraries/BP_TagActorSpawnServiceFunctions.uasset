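; Blueprint function library that spawns and links competency tag actors forming a hierarchy, using tag maps held in the BP_VariableStore game instance.
; It spawns a tag's children, or finds a tag's ancestor path recursively and spawns it downward from the roots, skipping existing or stored actors.
; Separate functions rebuild parent references and spawn connections for all actors.
; A helper picks a random sphere position with radius scaled by tag count.
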(fn GetRandomPositiononSphere
  (params (NumOfTags :type Integer))
  (bind _returnvalue (Math|Transform|MakeTransform))
  (LocalVariables|SetNumTags NumOfTags)
  (if (>= (LocalVariables|GetNumTags) 5)
    (LocalVariables|SetSphereRadius 100)
    (if (>= (LocalVariables|GetNumTags) 15)
      (LocalVariables|SetSphereRadius 150)
      (if (>= (LocalVariables|GetNumTags) 20)
        (LocalVariables|SetSphereRadius 200)
        (if (>= (LocalVariables|GetNumTags) 30)
          (LocalVariables|SetSphereRadius 300)
          (if (>= (LocalVariables|GetNumTags) 40)
            (LocalVariables|SetSphereRadius 400)
            (return _returnvalue)
            (else
              (return _returnvalue)))
          (else
            (return _returnvalue)))
        (else
          (return _returnvalue)))
      (else
        (return _returnvalue)))
    (else
      (return _returnvalue))))

(fn SpawnChildTags
  (params (TagActor :type ABP%20Tag%20Object%20Reference))
  (LocalVariables|SetParentActor TagActor)
  (|SetLocalVariables)
  (for _array_element (.children (.Value (Utilities|Map|Find (LocalVariables|GetTagChildren) (.id (Variables|/Game/Blueprints/TagActors/ABP_Tag.ABP_Tag_C|GetTag (LocalVariables|GetParentActor))))))
    (LocalVariables|SetTag _array_element)
    (if (not (.ReturnValue (Utilities|Map|Find (LocalVariables|GetTagActors) (.id (LocalVariables|GetTag)))))
      (bind _isstored (CallFunction|IsStoredTagActor (.id (LocalVariables|GetTag))))
      (if (not _isstored)
        (bind _spawnedtag (Default|SpawnTagActor (LocalVariables|GetParentActor) (LocalVariables|GetTag) (LocalVariables|GetParentActor)))
        (bind _output_get (LocalVariables|SetSpawnedChildTagActor _spawnedtag))
        (Utilities|Map|Add (LocalVariables|GetTagActors) (.id (Variables|/Game/Blueprints/TagActors/ABP_Tag.ABP_Tag_C|GetTag _output_get)) (LocalVariables|GetSpawnedChildTagActor))
        (Utilities|Array|AddUnique (Variables|/Game/Blueprints/TagActors/ABP_Tag.ABP_Tag_C|GetChildActors (LocalVariables|GetParentActor)) (LocalVariables|GetSpawnedChildTagActor)))))
  (|UpdateVariableStore)
  (return))

(fn IsStoredTagActor
  (params (TagID :type Integer))
  (bind _asbp_variable_store (Utilities|Casting|CastToBP_VariableStore (Game|GetGameInstance)))
  (for _array_element (Variables|/Game/Blueprints/BP_VariableStore.BP_VariableStore_C|GetStoredCompetencyActors _asbp_variable_store)
    (if (== (.id (Variables|/Game/Blueprints/TagActors/ABP_Tag.ABP_Tag_C|GetTag _array_element)) TagID)
      (LocalVariables|SetIsStoredActor true)))
  (return (LocalVariables|GetIsStoredActor)))

(fn SpawnPathTags
  (params (PathTagIDs :type Array%20of%20Integers))
  (bind _asbp_variable_store (Utilities|Casting|CastToBP_VariableStore (Game|GetGameInstance)))
  (for _array_element (Variables|/Game/Blueprints/BP_VariableStore.BP_VariableStore_C|GetRootCompetencies _asbp_variable_store)
    (if (.ReturnValue (Utilities|Map|Find (Variables|/Game/Blueprints/BP_VariableStore.BP_VariableStore_C|GetCompetenciesMap _asbp_variable_store) (.id _array_element)))
      (CallFunction|SpawnPathTagsRecursivly PathTagIDs (.id (.Value (Utilities|Map|Find (Variables|/Game/Blueprints/BP_VariableStore.BP_VariableStore_C|GetCompetenciesMap _asbp_variable_store) (.id _array_element))))))))

(fn SpawnPathTagsRecursivly
  (params (TagIDs :type Array%20of%20Integers) (Pivot :type Integer))
  (bind _pivottagactor (LocalVariables|GetPivotTagActor))
  (LocalVariables|SetCompetencyIDs TagIDs)
  (bind _output_get (LocalVariables|SetPivotID Pivot))
  (bind _isstored (CallFunction|IsStoredTagActor _output_get))
  (if _isstored
    (return)
    (else
      (bind _children (|GetChildrenOfPivot))
      (for _array_element _children
        (bind _output_get_2 (LocalVariables|SetChildID (.id _array_element)))
        (|IsInCompetencyIDs _output_get_2
          (:True
            (|ActorAlreadyExists
              (:True
                _)
              (:False
                (|SetPivotTagActor)
                (|SetChildTag)
                (bind _spawnedtag (Default|SpawnTagActor _pivottagactor (LocalVariables|GetChildTag) _pivottagactor))
                (|UpdateStore _spawnedtag)
                (Utilities|Array|AddUnique (Variables|/Game/Blueprints/TagActors/ABP_Tag.ABP_Tag_C|GetChildActors (LocalVariables|GetPivotTagActor)) _spawnedtag)))
            (CallFunction|SpawnPathTagsRecursivly (LocalVariables|GetCompetencyIDs) (LocalVariables|GetChildID)))))
      (return))))

(fn FindPathTags
  (params (TagID :type Integer))
  (bind _ids (CallFunction|FindPathTagsRecursivly TagID (Utilities|Array|MakeArray TagID)))
  (return _ids))

(fn FindPathTagsRecursivly
  (params (PivotID :type Integer) (PathTagIDs :type Array%20of%20Integers))
  (LocalVariables|SetTagID PivotID)
  (bind _output_get (LocalVariables|SetPathIDs PathTagIDs))
  (Utilities|Array|AddUnique _output_get (LocalVariables|GetTagID))
  (bind _asbp_variable_store (Utilities|Casting|CastToBP_VariableStore (Game|GetGameInstance)))
  (if (.ReturnValue (Utilities|Map|Find (Variables|/Game/Blueprints/BP_VariableStore.BP_VariableStore_C|GetCompetenciesParentsMap _asbp_variable_store) (LocalVariables|GetTagID)))
    (for _array_element (.parents (.Value (Utilities|Map|Find (Variables|/Game/Blueprints/BP_VariableStore.BP_VariableStore_C|GetCompetenciesParentsMap _asbp_variable_store) (LocalVariables|GetTagID))))
      (bind _ids (CallFunction|FindPathTagsRecursivly (.id _array_element) (LocalVariables|GetPathIDs)))
      (for _array_element_2 _ids
        (Utilities|Array|AddUnique (LocalVariables|GetPathIDs) _array_element_2))))
  (return (LocalVariables|GetPathIDs)))

(fn SetParentActorsOfAllTagActors
  (bind _asbp_variable_store (Utilities|Casting|CastToBP_VariableStore (Game|GetGameInstance)))
  (bind _keys (Utilities|Map|Keys (Variables|/Game/Blueprints/BP_VariableStore.BP_VariableStore_C|GetCompetencyActors _asbp_variable_store)))
  (for _array_element _keys
    (bind _output_get (LocalVariables|SetTagActor (.Value (Utilities|Map|Find (Variables|/Game/Blueprints/BP_VariableStore.BP_VariableStore_C|GetCompetencyActors _asbp_variable_store) _array_element))))
    (if (not (Variables|/Game/Blueprints/TagActors/ABP_Tag.ABP_Tag_C|GetisRoot _output_get))
      (Utilities|Array|Clear (Variables|/Game/Blueprints/TagActors/ABP_Tag.ABP_Tag_C|GetParentActors (LocalVariables|GetTagActor)))
      (bind _asbp_variable_store_2 (Utilities|Casting|CastToBP_VariableStore (Game|GetGameInstance)))
      (for _array_element_2 (.parents (.Value (Utilities|Map|Find (Variables|/Game/Blueprints/BP_VariableStore.BP_VariableStore_C|GetCompetenciesParentsMap _asbp_variable_store_2) (.id (Variables|/Game/Blueprints/TagActors/ABP_Tag.ABP_Tag_C|GetTag (LocalVariables|GetTagActor))))))
        (if (.ReturnValue (Utilities|Map|Find (Variables|/Game/Blueprints/BP_VariableStore.BP_VariableStore_C|GetCompetencyActors _asbp_variable_store_2) (.id _array_element_2)))
          (Utilities|Array|AddUnique (Variables|/Game/Blueprints/TagActors/ABP_Tag.ABP_Tag_C|GetParentActors (LocalVariables|GetTagActor)) (.Value (Utilities|Map|Find (Variables|/Game/Blueprints/BP_VariableStore.BP_VariableStore_C|GetCompetencyActors _asbp_variable_store_2) (.id _array_element_2))))))))
  (return))

(fn SpawnConnectionsOfAllTagActors
  (bind _asbp_variable_store (Utilities|Casting|CastToBP_VariableStore (Game|GetGameInstance)))
  (bind _keys (Utilities|Map|Keys (Variables|/Game/Blueprints/BP_VariableStore.BP_VariableStore_C|GetCompetencyActors _asbp_variable_store)))
  (for _array_element _keys
    (Default|SpawnConnections (.Value (Utilities|Map|Find (Variables|/Game/Blueprints/BP_VariableStore.BP_VariableStore_C|GetCompetencyActors _asbp_variable_store) _array_element))))
  (return))