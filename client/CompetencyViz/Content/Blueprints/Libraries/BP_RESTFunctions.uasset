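; Blueprint library of REST helpers that fetch and delete competency tags and their parent links on a backend server.
; Send functions build endpoints from the base URL in the BP_VariableStore game instance, fire VaRest GET or DELETE requests, and return the request and JSON objects.
; Separate response functions decode those objects, rebuilding the store's Competencies and CompetenciesParents arrays from parsed structs, or returning deleted tag IDs.
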(fn SendGetTagsRequest
  (bind _asbp_variable_store (Utilities|Casting|CastToBP_VariableStore (Game|GetGameInstance)))
  (bind (_json1 _request1) (CallFunction|SendGetRequest (Utilities|String|Append (Variables|/Game/Blueprints/BP_VariableStore.BP_VariableStore_C|GetURL _asbp_variable_store) "/tags")))
  (return _json1 _request1))

(fn SendGetRequest
  (params (URL :type String))
  (LocalVariables|SetJSON (Class|VaRestJsonObject|ConstructJsonObject))
  (bind _output_get (LocalVariables|SetRequest (Class|VaRestRequestJSON|ConstructRequestExt "GET" "x_www_form_urlencoded_url")))
  (Class|VaRestRequestJSON|GetRequestObject _output_get)
  (Class|VaRestRequestJSON|ProcessURL (LocalVariables|GetRequest) URL)
  (return (LocalVariables|GetJSON) (LocalVariables|GetRequest)))

(fn UpdateTagswithResponse
  (params (JSON :type Va%20Rest%20Json%20Object%20Object%20Reference) (Request :type Va%20Rest%20Request%20JSON%20Object%20Reference))
  (bind _returnvalue (CallFunction|GetArrayFieldfromJSON Request "tags" JSON))
  (bind _asbp_variable_store (Utilities|Casting|CastToBP_VariableStore (Game|GetGameInstance)))
  (Utilities|Array|Clear (Variables|/Game/Blueprints/BP_VariableStore.BP_VariableStore_C|GetCompetencies _asbp_variable_store))
  (for _array_element _returnvalue
    (bind _s_tag (CallFunction|GetTagfromJSON _array_element))
    (Utilities|Array|AddUnique (Variables|/Game/Blueprints/BP_VariableStore.BP_VariableStore_C|GetCompetencies _asbp_variable_store) _s_tag))
  (return))

(fn GetArrayFieldfromJSON
  (params (Request :type Va%20Rest%20Request%20JSON%20Object%20Reference) (FieldName :type String) (JSON :type Va%20Rest%20Json%20Object%20Object%20Reference))
  (bind _returnvalue (Class|VaRestRequestJSON|GetResponseContentasString Request true))
  (Class|VaRestJsonObject|DecodeJson JSON _returnvalue true)
  (return (Class|VaRestJsonObject|GetArrayField JSON FieldName)))

(fn GetTagfromJSON
  (params (JSON :type Va%20Rest%20Json%20Value%20Object%20Reference))
  (bind _returnvalue (Class|VaRestJsonValue|AsObject JSON))
  (return (Utilities|Struct|MakeS_Tag (Math|Conversions|ToInteger(Byte) (Class|VaRestJsonObject|GetStringField _returnvalue "id")) (.Result (Class|KismetMathLibrary|DateTimefromString (Class|VaRestJsonObject|GetStringField _returnvalue "created"))) (Class|VaRestJsonObject|GetStringField _returnvalue "created_by") (.Result (Class|KismetMathLibrary|DateTimefromString (Class|VaRestJsonObject|GetStringField _returnvalue "modified"))) (Class|VaRestJsonObject|GetStringField _returnvalue "modified_by") (Math|Conversions|ToInteger(Byte) (Class|VaRestJsonObject|GetStringField _returnvalue "version")) (Utilities|Text|ToText(String) (Class|VaRestJsonObject|GetStringField _returnvalue "description")) (Class|VaRestJsonObject|GetStringField _returnvalue "name") (Class|VaRestJsonObject|GetStringField _returnvalue "a_type"))))

(fn SendGetParentsRequest
  (bind _asbp_variable_store (Utilities|Casting|CastToBP_VariableStore (Game|GetGameInstance)))
  (bind (_json1 _request1) (CallFunction|SendGetRequest (Utilities|String|Append (Variables|/Game/Blueprints/BP_VariableStore.BP_VariableStore_C|GetURL _asbp_variable_store) "/tag-parents")))
  (return _json1 _request1))

(fn UpdateTagParentswithResponse
  (params (Request :type Va%20Rest%20Request%20JSON%20Object%20Reference) (JSON :type Va%20Rest%20Json%20Object%20Object%20Reference))
  (bind _returnvalue (CallFunction|GetArrayFieldfromJSON Request "tagParents" JSON))
  (bind _asbp_variable_store (Utilities|Casting|CastToBP_VariableStore (Game|GetGameInstance)))
  (Utilities|Array|Clear (Variables|/Game/Blueprints/BP_VariableStore.BP_VariableStore_C|GetCompetenciesParents _asbp_variable_store))
  (for _array_element _returnvalue
    (bind _s_tagparents (CallFunction|GetTagParentsfromJSON 0 _array_element))
    (Utilities|Array|AddUnique (Variables|/Game/Blueprints/BP_VariableStore.BP_VariableStore_C|GetCompetenciesParents _asbp_variable_store) _s_tagparents))
  (return))

(fn GetTagParentsfromJSON
  (params (JSON :type Va%20Rest%20Json%20Value%20Object%20Reference))
  (bind _returnvalue (Class|VaRestJsonValue|AsObject JSON))
  (return (Utilities|Struct|MakeS_TagParents (Math|Conversions|ToInteger(Byte) (Class|VaRestJsonObject|GetStringField _returnvalue "tag_id")) (Math|Conversions|ToInteger(Byte) (Class|VaRestJsonObject|GetStringField _returnvalue "parents_id")))))

(fn SendDeleteTagRequest
  (params (Tag :type S%20Tag%20Structure) (deleteChildren :type Boolean))
  (LocalVariables|SetTagID (.id Tag))
  (|CreateJSON deleteChildren)
  (bind _returnvalue (|CreateURL))
  (bind _request1 (CallFunction|SendDeleteRequest _returnvalue (LocalVariables|GetJSON)))
  (LocalVariables|SetRequest _request1)
  (return (LocalVariables|GetJSON) (LocalVariables|GetRequest)))

(fn SendDeleteRequest
  (params (URL :type String) (JSON :type Va%20Rest%20Json%20Object%20Object%20Reference))
  (bind _output_get (LocalVariables|SetRequest (Class|VaRestRequestJSON|ConstructRequestExt "DEL" "json")))
  (Class|VaRestRequestJSON|SetRequestObject _output_get JSON)
  (Class|VaRestRequestJSON|ProcessURL (LocalVariables|GetRequest) URL)
  (return (LocalVariables|GetRequest)))

(fn GetDeletedTagIdsfromJSON
  (params (Request :type Va%20Rest%20Request%20JSON%20Object%20Reference) (JSON :type Va%20Rest%20Json%20Object%20Object%20Reference))
  (bind _returnvalue (CallFunction|GetArrayFieldfromJSON Request "deletedTags" JSON))
  (for _array_element _returnvalue
    (bind _returnvalue_2 (Class|VaRestJsonValue|AsObject _array_element))
    (Utilities|Array|AddUnique (LocalVariables|GetDeletedTags) (Math|Conversions|ToInteger(Byte) (Class|VaRestJsonObject|GetStringField _returnvalue_2 "id"))))
  (return (LocalVariables|GetDeletedTags)))

(fn SendDeleteConnectionRequest
  (params (ChildTag :type S%20Tag%20Structure) (ParentTag :type S%20Tag%20Structure))
  (LocalVariables|SetChildID (.id ChildTag))
  (LocalVariables|SetParentID (.id ParentTag))
  (|CreateJSON)
  (bind _returnvalue (|CreateURL))
  (bind _request1 (CallFunction|SendDeleteRequest _returnvalue (LocalVariables|GetJSON)))
  (LocalVariables|SetRequest _request1)
  (return (LocalVariables|GetJSON) (LocalVariables|GetRequest)))