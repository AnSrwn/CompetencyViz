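; Blueprint color helper that hands out colors from a shared pool, cycling through all entries before reusing them.
; The pool lives in the BP_VariableStore game instance as color structs with an IsUsed flag.
; GetColor returns the first unused color, re-adding its entry as used and removing the original.
; When every color is used, ResetColorArray clears the flags and GetColor calls itself again.
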(fn GetColor
  (bind _asbp_variable_store (Utilities|Casting|CastToBP_VariableStore (Game|GetGameInstance)))
  (bind _output_get (LocalVariables|SetRootColors (Variables|/Game/Blueprints/BP_VariableStore.BP_VariableStore_C|GetColors _asbp_variable_store)))
  (for _array_element _output_get
    (if (not (.IsUsed (Utilities|Struct|BreakS_CategoryColor _array_element)))
      (Utilities|Array|Add (LocalVariables|GetRootColors) (Utilities|Struct|MakeS_CategoryColor (.Color (Utilities|Struct|BreakS_CategoryColor _array_element)) true))
      (Utilities|Array|RemoveItem (LocalVariables|GetRootColors) _array_element)
      (bind _asbp_variable_store_2 (Utilities|Casting|CastToBP_VariableStore (Game|GetGameInstance)))
      (Variables|/Game/Blueprints/BP_VariableStore.BP_VariableStore_C|SetColors _asbp_variable_store_2 (LocalVariables|GetRootColors))
      (return (.Color (Utilities|Struct|BreakS_CategoryColor _array_element)))))
  (|ResetColorArray _output_get)
  (bind _color (CallFunction|GetColor))
  (return _color))