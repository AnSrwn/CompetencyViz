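; BP_TagRecycleBin is a drop target that lets the player delete a grabbed tag actor.
; Overlap events on its collision box turn the cube red while the pawn's GrabbedTagActor is inside and white when it leaves, tracking this in a flag.
; On GrabbedTagActorReleased while overlapping, it opens WBP_DeleteTagDialog with that actor's tag, switches to UI-only input with a visible cursor and stops pawn movement.
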(event OnComponentBeginOverlap(CollisionBox)
  (params (OverlappedComponent :type Primitive%20Component%20Object%20Reference) (OtherActor :type Actor%20Object%20Reference) (OtherComp :type Primitive%20Component%20Object%20Reference) (OtherBodyIndex :type Integer) (bFromSweep :type Boolean) (SweepResult :type Hit%20Result%20Structure%20%28by%20ref%29))
  (bind _asbp_pawn (Utilities|Casting|CastToBP_Pawn (Game|Player|GetPlayerPawn 0)))
  (if (== (Variables|/Game/Blueprints/BP_Pawn.BP_Pawn_C|GetGrabbedTagActor _asbp_pawn) OtherActor)
    (Rendering|Material|SetMaterial (Variables|Default|GetCube) 0 "/Game/Materials/RedInlitMaterial.RedInlitMaterial")
    (Variables|Default|SetGrabbedTagActorIsOverlapping true)))

(event OnComponentEndOverlap(CollisionBox)
  (params (OverlappedComponent :type Primitive%20Component%20Object%20Reference) (OtherActor :type Actor%20Object%20Reference) (OtherComp :type Primitive%20Component%20Object%20Reference) (OtherBodyIndex :type Integer))
  (bind _asbp_pawn (Utilities|Casting|CastToBP_Pawn (Game|Player|GetPlayerPawn 0)))
  (if (== (Variables|/Game/Blueprints/BP_Pawn.BP_Pawn_C|GetGrabbedTagActor _asbp_pawn) OtherActor)
    (Variables|Default|SetGrabbedTagActorIsOverlapping false)
    (Rendering|Material|SetMaterial (Variables|Default|GetCube) 0 "/Game/Materials/WhiteInlitMaterial.WhiteInlitMaterial")))

(event Custom|GrabbedTagActorReleased
  (if (Variables|Default|GetGrabbedTagActorIsOverlapping)
    (bind _asbp_pawn (Utilities|Casting|CastToBP_Pawn (Game|Player|GetPlayerPawn 0)))
    (UserInterface|CreateWidget (Variables|/Game/Blueprints/BP_TagActor.BP_TagActor_C|GetTag (Variables|/Game/Blueprints/BP_Pawn.BP_Pawn_C|GetGrabbedTagActor _asbp_pawn)))))

(fn ConstructionScript)