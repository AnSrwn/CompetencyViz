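; Collision volume on the cable linking two tag actors, used to edit that connection.
; Touching the box opens a dialog to delete the connection.
; Overlap by the pawn's grabbed tag actor, gated by a check meant to exclude the connection's endpoints, opens a creation dialog with the child, new and parent tags.
; Both dialogs switch input to UI-only, show the cursor and stop pawn movement.
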(event OnInputTouchBegin(CollisionBox)
  (params (FingerIndex :type ETouchIndex%20Enum :default "Touch1") (TouchedComponent :type Primitive%20Component%20Object%20Reference))
  (CallFunction|OpenDeleteConnectionDialogWidget))

(event OnComponentBeginOverlap(CollisionBox)
  (params (OverlappedComponent :type Primitive%20Component%20Object%20Reference) (OtherActor :type Actor%20Object%20Reference) (OtherComp :type Primitive%20Component%20Object%20Reference) (OtherBodyIndex :type Integer) (bFromSweep :type Boolean) (SweepResult :type Hit%20Result%20Structure%20%28by%20ref%29))
  (bind _asbp_tag_actor (Utilities|Casting|CastToBP_TagActor OtherActor))
  (bind _asbp_pawn (Utilities|Casting|CastToBP_Pawn (Game|Player|GetPlayerPawn 0)))
  (if (== (Variables|/Game/Blueprints/BP_Pawn.BP_Pawn_C|GetGrabbedTagActor _asbp_pawn) _asbp_tag_actor)
    (if (|GrappedActorIsNotPartOfConnection _asbp_tag_actor)
      (UserInterface|CreateWidget (Variables|/Game/Blueprints/BP_TagActor.BP_TagActor_C|GetTag _asbp_tag_actor)))))

(fn ConstructionScript)

(fn OpenDeleteConnectionDialogWidget
  (bind _returnvalue (Game|GetPlayerController 0))
  (bind _connection (Variables|Default|GetConnection))
  (bind _returnvalue_2 (UserInterface|CreateWidget "/Game/Blueprints/Widgets/WBP_DeleteConnectionDialog.WBP_DeleteConnectionDialog_C" (Game|GetPlayerController 0) (Variables|/Game/Blueprints/BP_TagActor.BP_TagActor_C|GetTag (Variables|/Game/Blueprints/BP_ConnectionCable.BP_ConnectionCable_C|GetChildActor _connection)) (Variables|/Game/Blueprints/BP_TagActor.BP_TagActor_C|GetTag (Variables|/Game/Blueprints/BP_ConnectionCable.BP_ConnectionCable_C|GetParentActor _connection)) (Variables|Default|GetConnection)))
  (UserInterface|Viewport|AddtoViewport _returnvalue_2 0)
  (Input|SetInputModeUIOnly _returnvalue 0 "DoNotLock")
  (Variables|/Script/Engine.PlayerController|SetbShowMouseCursor _returnvalue true)
  (AI|Navigation|StopMovement))