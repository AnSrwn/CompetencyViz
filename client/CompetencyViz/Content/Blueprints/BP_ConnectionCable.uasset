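; BP_ConnectionCable is a cable actor that adds collision along the straight line between itself and its parent actor's TextRender.
; A gated Tick waits until the CableComponent's attached actor is valid, then builds the collision once.
; ActorMoved rebuilds it: destroy old boxes, then spawn and attach one BP_CollisionBoxForConnectionCable at the relative midpoint, oriented along the line and stretched to its length.
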(event Custom|EndPointActorIsValid
  (CallFunction|DestroyCollisionBoxes)
  (bind _returnvalue (CallFunction|GetVectorBetweenStartandEndPoint))
  (bind _returnvalue_2 (Game|SpawnActorfromClass "/Game/Blueprints/BP_CollisionBoxForConnectionCable.BP_CollisionBoxForConnectionCable_C" (Math|Transform|MakeTransform (* _returnvalue 0.5) (Math|Conversions|RotationFromXVector (Math|Vector|Normalize _returnvalue))) "AlwaysSpawn" 0 self 0))
  (Components|Box|SetBoxExtent (Variables|/Game/Blueprints/BP_CollisionBoxForConnectionCable.BP_CollisionBoxForConnectionCable_C|GetCollisionBox _returnvalue_2) (Math|Vector|MakeVector (* (Math|Vector|VectorLength _returnvalue) 0.5) 1.0 1.0) true)
  (Utilities|Array|Add (Variables|Default|GetCollisionBoxes) _returnvalue_2)
  (Transformation|AttachActorToActor _returnvalue_2 self "None" "KeepRelative" "KeepRelative" "KeepRelative" true))

(event Custom|ActorMoved
  (CallFunction|DestroyCollisionBoxes)
  (bind _returnvalue (CallFunction|GetVectorBetweenStartandEndPoint))
  (bind _returnvalue_2 (Game|SpawnActorfromClass "/Game/Blueprints/BP_CollisionBoxForConnectionCable.BP_CollisionBoxForConnectionCable_C" (Math|Transform|MakeTransform (* _returnvalue 0.5) (Math|Conversions|RotationFromXVector (Math|Vector|Normalize _returnvalue))) "AlwaysSpawn" 0 self 0))
  (Components|Box|SetBoxExtent (Variables|/Game/Blueprints/BP_CollisionBoxForConnectionCable.BP_CollisionBoxForConnectionCable_C|GetCollisionBox _returnvalue_2) (Math|Vector|MakeVector (* (Math|Vector|VectorLength _returnvalue) 0.5) 1.0 1.0) true)
  (Utilities|Array|Add (Variables|Default|GetCollisionBoxes) _returnvalue_2)
  (Transformation|AttachActorToActor _returnvalue_2 self "None" "KeepRelative" "KeepRelative" "KeepRelative" true))

(event EventTick
  (params (DeltaSeconds :type Float%20%28single-precision%29))
  (Utilities|FlowControl|Gate false :!label _label
    (:Exit
      (if (Utilities|IsValid (Class|CableComponent|GetAttachedActor (Variables|Default|GetCableComponent)))
        (CallFunction|EndPointActorIsValid)
        (goto _label Close)))))

(fn ConstructionScript)

(fn IsEven
  (params (Number :type Integer))
  (return (== (Math|Integer|%(Integer) Number 2) 0)))

(fn GetVectorBetweenStartandEndPoint
  (return (.location (Math|Transform|MakeRelativeTransform (Math|Conversions|ToTransform(Vector) (Transformation|GetWorldLocation (Variables|/Game/Blueprints/BP_TagActor.BP_TagActor_C|GetTextRender (Variables|Default|GetParentActor)))) (Transformation|GetActorTransform self)))))

(fn DestroyCollisionBoxes
  (for _array_element (Variables|Default|GetCollisionBoxes)
    (Actor|DestroyActor _array_element))
  (Utilities|Array|Clear (Variables|Default|GetCollisionBoxes))
  (return))