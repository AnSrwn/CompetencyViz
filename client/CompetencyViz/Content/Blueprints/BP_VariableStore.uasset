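; BP_VariableStore holds competency data and derives lookup structures for navigating its parent-child hierarchy.
; UpdateVariableStore rebuilds everything in order, starting with an Id-to-competency map from the Competencies array.
; That map resolves CompetenciesParents ID pairs into parents-per-tag and children-per-parent maps, using struct wrappers to store arrays as map values.
; Root competencies are those that never appear as a child in the pairs.
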(fn UpdateCompetenciesMap
  (Utilities|Map|Clear (Variables|Default|GetCompetenciesMap))
  (for _array_element (Variables|Default|GetCompetencies)
    (Utilities|Map|Add (Variables|Default|GetCompetenciesMap) (.Id (Utilities|Struct|BreakS_Tag _array_element)) _array_element))
  (return))

(fn UpdateCompetenciesParentsMap
  (Utilities|Map|Clear (Variables|Default|GetCompetenciesParentsMap))
  (for _array_element (Variables|Default|GetCompetenciesParents)
    (LocalVariables|SetTagID (.tagid _array_element))
    (LocalVariables|SetParentID (.parentsid _array_element))
    (LocalVariables|SetParents (.parents (.Value (Utilities|Map|Find (Variables|Default|GetCompetenciesParentsMap) (LocalVariables|GetTagID)))))
    (if (.ReturnValue (Utilities|Map|Find (Variables|Default|GetCompetenciesParentsMap) (LocalVariables|GetTagID)))
      (Utilities|Array|Add (LocalVariables|GetParents) (.Value (Utilities|Map|Find (Variables|Default|GetCompetenciesMap) (LocalVariables|GetParentID))))
      (Utilities|Map|Add (Variables|Default|GetCompetenciesParentsMap) (LocalVariables|GetTagID) (Utilities|Struct|MakeS_TagParentsForMap (LocalVariables|GetParents)))
      (else
        (Utilities|Map|Add (Variables|Default|GetCompetenciesParentsMap) (LocalVariables|GetTagID) (Utilities|Struct|MakeS_TagParentsForMap (Utilities|Array|MakeArray (.Value (Utilities|Map|Find (Variables|Default|GetCompetenciesMap) (LocalVariables|GetParentID)))))))))
  (return))

(fn UpdateCompetenciesChildren
  (Utilities|Map|Clear (Variables|Default|GetCompetenciesChildren))
  (for _array_element (Variables|Default|GetCompetenciesParents)
    (LocalVariables|SetTagID (.tagid _array_element))
    (LocalVariables|SetParentID (.parentsid _array_element))
    (bind _output_get (LocalVariables|SetTagChildren (.Value (Utilities|Map|Find (Variables|Default|GetCompetenciesChildren) (LocalVariables|GetParentID)))))
    (Utilities|Array|AddUnique (.children _output_get) (.Value (Utilities|Map|Find (Variables|Default|GetCompetenciesMap) (LocalVariables|GetTagID))))
    (Utilities|Map|Add (Variables|Default|GetCompetenciesChildren) (LocalVariables|GetParentID) (LocalVariables|GetTagChildren)))
  (return))

(fn UpdateVariableStore
  (CallFunction|UpdateCompetenciesMap)
  (CallFunction|UpdateCompetenciesParentsMap)
  (CallFunction|UpdateCompetenciesChildren)
  (CallFunction|UpdateRootCompetencies))

(fn UpdateRootCompetencies
  (Utilities|Array|Clear (Variables|Default|GetRootCompetencies))
  (for _array_element (Variables|Default|GetCompetenciesParents)
    (Utilities|Map|Add (LocalVariables|GetTagsWithParents) (.tagid _array_element) (.parentsid _array_element)))
  (for _array_element_2 (Variables|Default|GetCompetencies)
    (if (not (.ReturnValue (Utilities|Map|Find (LocalVariables|GetTagsWithParents) (.Id (Utilities|Struct|BreakS_Tag _array_element_2)))))
      (Utilities|Array|AddUnique (Variables|Default|GetRootCompetencies) _array_element_2)))
  (return))