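; Touchable 3D text node for one competency tag in a graph whose data and actor registry live in BP_VariableStore.
; Single tap prunes to roots and ancestors, then spawns children; double tap recursively reveals related ancestors and descendants, linked by beam emitters.
; A timer-based long press hands movement to BP_Pawn.
; Each tick, text faces the camera and overlapping tags nudge apart with randomized interpolation.
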(event EventBeginPlay
  (|SetNumOfChildren)
  (Rendering|Components|TextRender|SetText)
  (|SetTextColor)
  (|SetSizeOfText)
  (Components|Sphere|SetSphereRadius)
  (CallFunction|SetParentActors)
  (CallFunction|SetHasHiddenChildrenIndicator))

(event EventActorOnInputTouchEnd
  (params (FingerIndex :type ETouchIndex%20Enum :default "Touch1"))
  (if (|IsLongTouch)
    (Utilities|Time|ClearandInvalidateTimerbyHandle (Variables|Default|GetTimeHandler))
    (CallFunction|StopMovingTagActor)
    (else
      (Utilities|Time|ClearandInvalidateTimerbyHandle (Variables|Default|GetTimeHandler))
      (Utilities|IsDoubleClick
        (:Double
          (CallFunction|ShowDetailsOfTag))
        (:Single
          (CallFunction|ShowChildTags))))))

(event EventActorOnInputTouchBegin
  (params (FingerIndex :type ETouchIndex%20Enum :default "Touch1"))
  (bind _returnvalue (Utilities|Time|SetTimerbyFunctionName 0 "MoveTagActor" 0.75))
  (Variables|Default|SetTimeHandler _returnvalue))

(event EventTick
  (params (DeltaSeconds :type Float%20%28single-precision%29))
  (bind _rotation (CallFunction|GetNewRotationforTextRender))
  (Transformation|SetWorldRotation (Variables|Default|GetTextRender) _rotation false false)
  (bind _returnvalue (CallFunction|IsOverlappedbyOtherActors))
  (if _returnvalue
    (CallFunction|MoveAwayfromOverlappingActors)))

(fn ConstructionScript)

(fn SetTextSize
  (params (TextRender :type Text%20Render%20Component%20Object%20Reference))
  (LocalVariables|SetText TextRender)
  (if (>= (Variables|Default|GetNumOfChildren) 10)
    (Rendering|Components|TextRender|SetWorldSize (LocalVariables|GetText) 15.0)
    (if (>= (Variables|Default|GetNumOfChildren) 30)
      (Rendering|Components|TextRender|SetWorldSize (LocalVariables|GetText) 2e+01)
      (return (LocalVariables|GetText))
      (else
        (return (LocalVariables|GetText))))
    (else
      (return (LocalVariables|GetText)))))

(fn DestroyUnnecessaryTagActors
  (params (NecessaryTagIDs :type Array%20of%20Integers))
  (LocalVariables|SetNecessaryCompetencyIDs NecessaryTagIDs)
  (bind _asbp_variable_store (Utilities|Casting|CastToBP_VariableStore (Game|GetGameInstance)))
  (LocalVariables|SetCompetencyActors (Variables|/Game/Blueprints/BP_VariableStore.BP_VariableStore_C|GetCompetencyActors _asbp_variable_store))
  (bind _output_get (LocalVariables|SetCompetencies (Variables|/Game/Blueprints/BP_VariableStore.BP_VariableStore_C|GetCompetencies _asbp_variable_store)))
  (for _array_element _output_get
    (LocalVariables|SetPotentialActorToDelete (.Value (Utilities|Map|Find (LocalVariables|GetCompetencyActors) (.id _array_element))))
    (if (.ReturnValue (Utilities|Map|Find (LocalVariables|GetCompetencyActors) (.id _array_element)))
      (if (not (>= (Utilities|Array|FindItem (LocalVariables|GetNecessaryCompetencyIDs) (.id _array_element)) 0))
        (for _array_element_2 (Variables|BP_TagActor_C|GetConnections (LocalVariables|GetPotentialActorToDelete))
          (Components|Activation|Deactivate _array_element_2))
        (Utilities|Array|RemoveItem (Variables|Default|GetChildActors) (LocalVariables|GetPotentialActorToDelete))
        (Utilities|Map|Remove (LocalVariables|GetCompetencyActors) (.id (Variables|BP_TagActor_C|GetTag (LocalVariables|GetPotentialActorToDelete))))
        (Actor|DestroyActor (LocalVariables|GetPotentialActorToDelete)))))
  (bind _asbp_variable_store_2 (Utilities|Casting|CastToBP_VariableStore (Game|GetGameInstance)))
  (Variables|/Game/Blueprints/BP_VariableStore.BP_VariableStore_C|SetCompetencyActors _asbp_variable_store_2 (LocalVariables|GetCompetencyActors)))

(fn SpawnChildTags
  (bind _color (Variables|Default|GetColor))
  (bind _output_get (|SetLocalVariables))
  (if (.ReturnValue (Utilities|Map|Find _output_get (.id (Variables|Default|GetTag))))
    (for _array_element (.children (.Value (Utilities|Map|Find _output_get (.id (Variables|Default|GetTag)))))
      (bind _output_get_2 (LocalVariables|SetCompetency _array_element))
      (if (> (Utilities|String|Len (.Name (Utilities|Struct|BreakS_Tag _output_get_2))) 0)
        (if (not (.ReturnValue (Utilities|Map|Find (LocalVariables|GetCompetencyActors) (.Id (Utilities|Struct|BreakS_Tag (LocalVariables|GetCompetency))))))
          (bind _returnvalue (CallFunction|GetRandomTransformonCircleOfTag))
          (bind _returnvalue_2 (Game|SpawnActorfromClass "BP_TagActor_C" _returnvalue "AdjustIfPossibleButAlwaysSpawn" 0 (LocalVariables|GetCompetency) false (Utilities|Struct|MakeS_Color (.r _color) (.g _color) (.b _color) (- (.a _color) 20)) self 0))
          (Transformation|AttachActorToActor _returnvalue_2 self "None" "KeepRelative" "KeepRelative" "KeepRelative" true)
          (bind _output_get_3 (LocalVariables|SetNewChildTagActor _returnvalue_2))
          (Utilities|Map|Add (LocalVariables|GetCompetencyActors) (.id (Variables|BP_TagActor_C|GetTag _output_get_3)) (LocalVariables|GetNewChildTagActor))
          (Utilities|Array|Add (Variables|Default|GetChildActors) (LocalVariables|GetNewChildTagActor)))))
    (|UpdateVariableStore)
    (return)))

(fn FindAllNecessaryParentTags
  (params (TagID :type Integer) (Ids :type Array%20of%20Integers))
  (bind _output_get (LocalVariables|SetIDsOfAllNecessaryTags Ids))
  (Utilities|Array|AddUnique _output_get TagID)
  (bind _asbp_variable_store (Utilities|Casting|CastToBP_VariableStore (Game|GetGameInstance)))
  (if (.ReturnValue (Utilities|Map|Find (Variables|/Game/Blueprints/BP_VariableStore.BP_VariableStore_C|GetCompetenciesParentsMap _asbp_variable_store) TagID))
    (for _array_element (.parents (.Value (Utilities|Map|Find (Variables|/Game/Blueprints/BP_VariableStore.BP_VariableStore_C|GetCompetenciesParentsMap _asbp_variable_store) TagID)))
      (bind _tagids (CallFunction|FindAllNecessaryParentTags (.id _array_element) (LocalVariables|GetIDsOfAllNecessaryTags)))
      (for _array_element_2 _tagids
        (Utilities|Array|AddUnique (LocalVariables|GetIDsOfAllNecessaryTags) _array_element_2))))
  (return (LocalVariables|GetIDsOfAllNecessaryTags)))

(fn SetInitalNecessaryTagIDs
  (Utilities|Array|AddUnique (LocalVariables|GetNecessaryTagIDs) (.id (Variables|Default|GetTag)))
  (bind _asbp_variable_store (Utilities|Casting|CastToBP_VariableStore (Game|GetGameInstance)))
  (for _array_element (Variables|/Game/Blueprints/BP_VariableStore.BP_VariableStore_C|GetRootCompetencies _asbp_variable_store)
    (Utilities|Array|AddUnique (LocalVariables|GetNecessaryTagIDs) (.id _array_element)))
  (return (LocalVariables|GetNecessaryTagIDs)))

(fn GetRandomTransformonCircleOfTag
  (bind _returnvalue (Math|Random|RandomUnitVector))
  (return (Math|Transform|MakeTransform (+ (* (Math|Vector|MakeVector (.x _returnvalue) (.y _returnvalue) (.z _returnvalue)) (Math|Random|RandomFloatinRange 5e+01 3e+02)) (Variables|/Script/Engine.SceneComponent|GetRelativeLocation (Variables|Default|GetOverlapSphere))))))

(fn GetNewRotationforTextRender
  (bind _asbp_pawn (Utilities|Casting|CastToBP_Pawn (Game|Player|GetPlayerPawn 0)))
  (return (Math|Rotator|FindLookatRotation (Transformation|GetWorldLocation (Variables|Default|GetTextRender)) (Transformation|GetWorldLocation (Variables|/Game/Blueprints/BP_Pawn.BP_Pawn_C|GetCamera _asbp_pawn)))))

(fn GetDirectionVector
  (bind _overlapsphere (Variables|Default|GetOverlapSphere))
  (bind _spawnparentactor (Variables|Default|GetSpawnParentActor))
  (bind _returnvalue (Transformation|GetWorldLocation _overlapsphere))
  (bind _asbp_tag_actor (Utilities|Casting|CastToBP_TagActor _spawnparentactor)
    (:then
      (LocalVariables|SetWorldLocationOfParent (Transformation|GetWorldLocation (Variables|BP_TagActor_C|GetOverlapSphere _asbp_tag_actor))))
    (:CastFailed
      (bind _asbp_anchor_actor (Utilities|Casting|CastToBP_AnchorActor _spawnparentactor))
      (LocalVariables|SetWorldLocationOfParent (Transformation|GetWorldLocation (Variables|/Game/Blueprints/BP_AnchorActor.BP_AnchorActor_C|GetStaticMesh _asbp_anchor_actor)))))
  (return (Math|Vector|MakeVector (.x (+ (Math|Vector|Normalize (- (LocalVariables|GetWorldLocationOfParent) _returnvalue)) _returnvalue)) (.y (+ (Math|Vector|Normalize (- (LocalVariables|GetWorldLocationOfParent) _returnvalue)) _returnvalue)) (Math|Random|RandomFloatinRange 0.0 0.5))))

(fn IsOverlappedbyOtherActors
  (return (> (Utilities|Array|Length (Collision|GetOverlappingActors (Variables|Default|GetOverlapSphere) "BP_TagActor_C" :!class /Script/Engine.PrimitiveComponent)) 0)))

(fn GetNewLocation
  (bind _returnvalue (CallFunction|GetDirectionVector))
  (return (Math|Interpolation|VInterpTo (Transformation|GetWorldLocation (Variables|Default|GetDefaultSceneRoot)) (* _returnvalue (Math|Random|RandomFloatinRange 1.0 1.3)) (Utilities|Time|GetWorldDeltaSeconds) (Math|Random|RandomFloatinRange 0.0 1e+01))))

(fn MoveAwayfromOverlappingActors
  (if (Utilities|IsValid (Variables|Default|GetSpawnParentActor))
    (for _array_element (Collision|GetOverlappingActors (Variables|Default|GetOverlapSphere) "BP_TagActor_C" :!class /Script/Engine.PrimitiveComponent)
      (bind _asbp_tag_actor (Utilities|Casting|CastToBP_TagActor _array_element))
      (if (not (|ShouldNotMove _asbp_tag_actor _asbp_tag_actor))
        (bind _returnvalue (CallFunction|GetNewLocation))
        (Transformation|SetWorldLocation (Variables|Default|GetDefaultSceneRoot) _returnvalue false false)))
    (return)))

(fn DrawLinestoParentActors
  (for _array_element (Variables|Default|GetParentActors)
    (bind _returnvalue (Effects|SpawnEmitteratLocation "/Game/ParticleSystem/BeamConnection.BeamConnection" "0, 0, 0"))
    (Effects|Components|ParticleSystem|SetActorParameter _returnvalue "BeamSource" self)
    (Effects|Components|ParticleSystem|SetActorParameter _returnvalue "BeamTarget" _array_element)
    (Utilities|Array|Add (Variables|Default|GetConnections) _returnvalue))
  (return))

(fn ShowDetailsOfTag
  (bind _ids (CallFunction|SetInitalNecessaryTagIDs))
  (bind _tagids (CallFunction|FindAllNecessaryParentTags (.id (Variables|Default|GetTag)) _ids))
  (LocalVariables|SetNecessaryTagIDs _tagids)
  (bind _tagids_2 (CallFunction|FindAllNecessaryChildrenTags (.id (Variables|Default|GetTag))))
  (for _array_element _tagids_2
    (Utilities|Array|AddUnique (LocalVariables|GetNecessaryTagIDs) _array_element))
  (CallFunction|DestroyUnnecessaryTagActors (LocalVariables|GetNecessaryTagIDs))
  (bind _asbp_variable_store (Utilities|Casting|CastToBP_VariableStore (Game|GetGameInstance)))
  (for _array_element_2 (LocalVariables|GetNecessaryTagIDs)
    (if (.ReturnValue (Utilities|Map|Find (Variables|/Game/Blueprints/BP_VariableStore.BP_VariableStore_C|GetCompetencyActors _asbp_variable_store) _array_element_2))
      (if (Variables|BP_TagActor_C|GetisRoot (.Value (Utilities|Map|Find (Variables|/Game/Blueprints/BP_VariableStore.BP_VariableStore_C|GetCompetencyActors _asbp_variable_store) _array_element_2)))
        (CallFunction|SpawnNecessaryTags (LocalVariables|GetNecessaryTagIDs) _array_element_2))))
  (|SetParentActorsOfNecessaryActors)
  (|DrawLinwsOfNecessaryActors))

(fn FindAllNecessaryChildrenTags
  (params (TagID :type Integer))
  (LocalVariables|SetID TagID)
  (bind _asbp_variable_store (Utilities|Casting|CastToBP_VariableStore (Game|GetGameInstance)))
  (LocalVariables|SetChildrenArray (.children (.Value (Utilities|Map|Find (Variables|/Game/Blueprints/BP_VariableStore.BP_VariableStore_C|GetCompetenciesChildren _asbp_variable_store) (LocalVariables|GetID)))))
  (if (.ReturnValue (Utilities|Map|Find (Variables|/Game/Blueprints/BP_VariableStore.BP_VariableStore_C|GetCompetenciesChildren _asbp_variable_store) (LocalVariables|GetID)))
    (for _array_element (LocalVariables|GetChildrenArray)
      (bind _tagids (CallFunction|FindAllNecessaryChildrenTags (.id _array_element)))
      (for _array_element_2 _tagids
        (Utilities|Array|AddUnique (LocalVariables|GetAllNecessaryChildrenTagIDs) _array_element_2)))
    (else
      (Utilities|Array|AddUnique (LocalVariables|GetAllNecessaryChildrenTagIDs) (LocalVariables|GetID))))
  (return (LocalVariables|GetAllNecessaryChildrenTagIDs)))

(fn SpawnNecessaryTags
  (params (NecessaryTagIDs :type Array%20of%20Integers) (TagID :type Integer))
  (LocalVariables|SetNecessaryTags NecessaryTagIDs)
  (LocalVariables|SetID TagID)
  (bind _asbp_variable_store (Utilities|Casting|CastToBP_VariableStore (Game|GetGameInstance)))
  (if (.ReturnValue (Utilities|Map|Find (Variables|/Game/Blueprints/BP_VariableStore.BP_VariableStore_C|GetCompetenciesChildren _asbp_variable_store) (LocalVariables|GetID)))
    (for _array_element (.children (.Value (Utilities|Map|Find (Variables|/Game/Blueprints/BP_VariableStore.BP_VariableStore_C|GetCompetenciesChildren _asbp_variable_store) (LocalVariables|GetID))))
      (bind _output_get (LocalVariables|SetChildID (.id _array_element)))
      (if (>= (Utilities|Array|FindItem (LocalVariables|GetNecessaryTags) _output_get) 0)
        (bind _asbp_variable_store_2 (Utilities|Casting|CastToBP_VariableStore (Game|GetGameInstance)))
        (bind _output_get_2 (LocalVariables|SetCompetencyActors (Variables|/Game/Blueprints/BP_VariableStore.BP_VariableStore_C|GetCompetencyActors _asbp_variable_store_2)))
        (if (.ReturnValue (Utilities|Map|Find _output_get_2 (LocalVariables|GetChildID)))
          (CallFunction|SpawnNecessaryTags (LocalVariables|GetNecessaryTags) (LocalVariables|GetChildID))
          (else
            (bind _returnvalue (CallFunction|GetRandomTransformonCircleOfTag (.Value (Utilities|Map|Find (LocalVariables|GetCompetencyActors) (LocalVariables|GetID)))))
            (bind _returnvalue_2 (Game|SpawnActorfromClass "BP_TagActor_C" _returnvalue "AdjustIfPossibleButAlwaysSpawn" 0 (.Value (Utilities|Map|Find (Variables|/Game/Blueprints/BP_VariableStore.BP_VariableStore_C|GetCompetenciesMap _asbp_variable_store_2) (LocalVariables|GetChildID))) false (Variables|BP_TagActor_C|GetColor (.Value (Utilities|Map|Find (LocalVariables|GetCompetencyActors) (LocalVariables|GetID)))) (.Value (Utilities|Map|Find (LocalVariables|GetCompetencyActors) (LocalVariables|GetID))) 0))
            (Utilities|Map|Add (LocalVariables|GetCompetencyActors) (LocalVariables|GetChildID) _returnvalue_2)
            (bind _asbp_variable_store_3 (Utilities|Casting|CastToBP_VariableStore (Game|GetGameInstance)))
            (Variables|/Game/Blueprints/BP_VariableStore.BP_VariableStore_C|SetCompetencyActors _asbp_variable_store_3 (LocalVariables|GetCompetencyActors))
            (CallFunction|SpawnNecessaryTags (LocalVariables|GetNecessaryTags) (LocalVariables|GetChildID))))))
    (return)
    (else
      (return))))

(fn SetParentActors
  (bind _asbp_variable_store (Utilities|Casting|CastToBP_VariableStore (Game|GetGameInstance)))
  (for _array_element (.parents (.Value (Utilities|Map|Find (Variables|/Game/Blueprints/BP_VariableStore.BP_VariableStore_C|GetCompetenciesParentsMap _asbp_variable_store) (.id (Variables|Default|GetTag)))))
    (if (.ReturnValue (Utilities|Map|Find (Variables|/Game/Blueprints/BP_VariableStore.BP_VariableStore_C|GetCompetencyActors _asbp_variable_store) (.id _array_element)))
      (Utilities|Array|Add (Variables|Default|GetParentActors) (.Value (Utilities|Map|Find (Variables|/Game/Blueprints/BP_VariableStore.BP_VariableStore_C|GetCompetencyActors _asbp_variable_store) (.id _array_element))))))
  (return))

(fn SetHasHiddenChildrenIndicator
  (Rendering|SetVisibility (Variables|Default|GetHasHiddenChildrenIndicator) (not (>= (Utilities|Array|Length (Variables|Default|GetChildActors)) (Variables|Default|GetNumOfChildren))) false)
  (return))

(fn MoveTagActor
  (bind _asbp_pawn (Utilities|Casting|CastToBP_Pawn (Game|Player|GetPlayerPawn 0)))
  (Default|MoveTagActor _asbp_pawn self))

(fn StopMovingTagActor
  (bind _asbp_pawn (Utilities|Casting|CastToBP_Pawn (Game|Player|GetPlayerPawn 0)))
  (Default|StopMovingTagActor _asbp_pawn))

(fn ShowChildTags
  (|PrintIfThereAreChildTags)
  (bind _ids (CallFunction|SetInitalNecessaryTagIDs))
  (bind _tagids (CallFunction|FindAllNecessaryParentTags (.id (Variables|Default|GetTag)) _ids))
  (CallFunction|DestroyUnnecessaryTagActors _tagids)
  (CallFunction|SpawnChildTags)
  (CallFunction|SetHasHiddenChildrenIndicator))